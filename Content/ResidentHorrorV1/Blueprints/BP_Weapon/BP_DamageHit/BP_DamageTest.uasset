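; BP_DamageTest is a mannequin target for testing weapon damage that ragdolls on death and spawns a replacement.
; EventDamage subtracts damage from Health while alive, then checks Health minus Damage to set Dead.
; On death, the skeletal mesh simulates physics and its head bone gets a velocity-change impulse along the shot direction.
; One second later a new copy spawns at the actor's transform, without destroying the old one.
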(event EventBeginPlay)

(event Collision|EventActorBeginOverlap
  (params (OtherActor :type Actor%20Object%20Reference)))

(event EventTick
  (params (DeltaSeconds :type Float%20%28single-precision%29)))

(event EventEventDamage
  (params (Damage :type Float%20%28double-precision%29) (HitResult :type Hit%20Result%20Structure))
  (bind (_bblockinghit _binitialoverlap _time _distance _location _impactpoint _normal _impactnormal _physmat _hitactor _hitcomponent _hitbonename _bonename _hititem _elementindex _faceindex _tracestart) (Collision|BreakHitResult HitResult))
  ;[0 0 0] Matar mannequin
  (if (not (Variables|Default|GetDead?))
    (Variables|Default|SetHealth (- (Variables|Default|GetHealth) Damage))
    (if (<= (- (Variables|Default|GetHealth) Damage) 0.0)
      (Variables|Default|SetDead? true)
      (Physics|SetSimulatePhysics (Variables|Default|GetSkeletalMesh) true)
      (Physics|AddImpulse (Variables|Default|GetSkeletalMesh) (* (Math|Vector|Normalize (- _impactpoint _tracestart) 5.0) 1.85e+04) "head" true)
      (Utilities|FlowControl|Delay 1.0)
      (Game|SpawnActorfromClass "BP_DamageTest_C" (Transformation|GetActorTransform) "Undefined" "MultiplyWithRoot" 0 0))))

(fn ConstructionScript)